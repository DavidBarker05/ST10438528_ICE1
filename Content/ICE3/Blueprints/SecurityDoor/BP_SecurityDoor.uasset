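; BP_SecurityDoor is a keypad-locked door that slides open when a character enters the correct code.
; A StandPosition overlap gates InputButtonValue, which appends each button value to CurrentCode while input is allowed.
; Once the length matches CorrectCode, a match locks input and opens the door, while a mismatch resets the code to "-".
; A timeline lerps the door from its start along its negative right vector.
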(event `self.ReceiveBeginPlay`
  (bind _output_get (set `self.DoorStart` (`SceneComponent.K2_GetComponentLocation` (`self.Door`))))
  (set `self.DoorEnd` (- _output_get (* (`self.DoorMoveDistance`) (`SceneComponent.GetRightVector` (`self.Door`))))))

(event `Event OpenDoor`
  (bind (_direction _doorlerp) (`Timeline|Open Door`)
    (:`Update`
      (`SceneComponent.K2_SetWorldLocation` (`self.Door`) (`KismetMathLibrary.VLerp` (`self.DoorStart`) (`self.DoorEnd`) _doorlerp) false false))))

(event `self.Stand Position.OnComponentBeginOverlap`
  (params (OverlappedComponent :type "PrimitiveComponent Object Reference") (OtherActor :type "Actor Object Reference") (OtherComp :type "PrimitiveComponent Object Reference") (OtherBodyIndex :type Integer) (bFromSweep :type Boolean) (SweepResult :type "HitResult Structure (by ref)"))
  (cast `Character` OtherActor)
  (set `self.IsPlayerInBox` true))

(event `self.Stand Position.OnComponentEndOverlap`
  (params (OverlappedComponent :type "PrimitiveComponent Object Reference") (OtherActor :type "Actor Object Reference") (OtherComp :type "PrimitiveComponent Object Reference") (OtherBodyIndex :type Integer))
  (cast `Character` OtherActor)
  (set `self.IsPlayerInBox` false))

(fn `InputButtonValue`
  (params (ButtonValue :type Byte))
  (if (and (`self.CanInputCode`) (`self.IsPlayerInBox`))
    (bind _output_get (set `self.CurrentCode` (`KismetTextLibrary.Conv_StringToText` (`KismetStringLibrary.Concat_StrStr` (`KismetTextLibrary.Conv_TextToString` (`self.CurrentCode`)) (`KismetStringLibrary.Conv_ByteToString` ButtonValue)))))
    (if (== (`KismetStringLibrary.Len` (`KismetTextLibrary.Conv_TextToString` _output_get)) (`KismetStringLibrary.Len` (`KismetTextLibrary.Conv_TextToString` (`self.CorrectCode`))))
      (if (`KismetStringLibrary.EqualEqual_StrStr` (`KismetTextLibrary.Conv_TextToString` (`self.CurrentCode`)) (`KismetTextLibrary.Conv_TextToString` (`self.CorrectCode`)))
        (set `self.CanInputCode` false)
        (`self.Event OpenDoor`)
        (else
          (set `self.CurrentCode` "-"))))))

(fn `UserConstructionScript`)