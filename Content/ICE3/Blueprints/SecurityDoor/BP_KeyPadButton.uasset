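; BP_KeyPadButton is a numbered keypad button that feeds digit input to a BP_SecurityDoor.
; The construction script shows its DisplayNumber on a text render component.
; On BeginPlay it caches its parent actor as the owning security door, and PressButton passes DisplayNumber to that door's InputButtonValue when the door is valid.
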(event `self.ReceiveBeginPlay`
  (bind _asbp_security_door (cast `/Game/ICE3/Blueprints/SecurityDoor/BP_SecurityDoor` (`self.GetParentActor`)))
  (set `self.OwningSecurityDoor` _asbp_security_door))

(fn `PressButton`
  (bind _owningsecuritydoor (`self.OwningSecurityDoor`))
  (`/Engine/EditorBlueprintResources/StandardMacros.IsValid` _owningsecuritydoor
    (:`Is Valid`
      (`/Game/ICE3/Blueprints/SecurityDoor/BP_SecurityDoor.InputButtonValue` _owningsecuritydoor (`self.DisplayNumber`)))))

(fn `UserConstructionScript`
  (`TextRenderComponent.K2_SetText` (`self.TextRender`) (`KismetTextLibrary.Conv_ByteToText` (`self.DisplayNumber`))))